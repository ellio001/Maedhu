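; Flying crow obstacle that loads the Game_Over level when it registers a hit and expires after a fixed lifespan.
; Tick steps the actor along negative X and up or down, branching on stored height values, with debug prints per branch.
; Z, ZMax and ZMin all hold the spawn height and never update, so it only climbs rather than oscillating.
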(event EventBeginPlay
  (bind _returnvalue (Transformation|GetActorLocation))
  (Variables|Default|SetZ (.z _returnvalue))
  (bind _output_get (Variables|Default|SetZ_Max (.z _returnvalue)))
  (bind _output_get_2 (Variables|Default|SetZ_Min (.z _returnvalue)))
  (Actor|SetLifeSpan 2e+01) ; 寿命
)

(event Collision|EventActorBeginOverlap
  (params (OtherActor :type Actor%20Object%20Reference)))

(event EventTick
  (params (DeltaSeconds :type Float%20%28single-precision%29))
  (bind _returnvalue (Transformation|GetActorLocation))
  (bind _returnvalue_2 (Transformation|GetActorLocation))
  (if (>= (Variables|Default|GetZ) (Variables|Default|GetZ_Max))
    (Development|PrintString "A")
    (Transformation|SetActorLocation (Math|Vector|MakeVector (- (.x _returnvalue) 1e+01) (.y _returnvalue) (+ (.z _returnvalue) 1e+01)) false false :!label _label) ; 移動
    (else
      (Development|PrintString "B")
      (if (>= (Variables|Default|GetZ_Min) (Variables|Default|GetZ))
        (Development|PrintString "A_2")
        (goto _label)
        (else
          (Development|PrintString "B_2")
          (Transformation|SetActorLocation (Math|Vector|MakeVector (- (.x _returnvalue_2) 1e+01) (.y _returnvalue_2) (- (.z _returnvalue_2) 1e+01)) false false) ; 移動
        )))))

(event Collision|EventHit
  (params (MyComp :type Primitive%20Component%20Object%20Reference) (Other :type Actor%20Object%20Reference) (OtherComp :type Primitive%20Component%20Object%20Reference) (bSelfMoved :type Boolean) (HitLocation :type Vector :default "0, 0, 0") (HitNormal :type Vector :default "0, 0, 0") (NormalImpulse :type Vector :default "0, 0, 0") (Hit :type Hit%20Result%20Structure%20%28by%20ref%29))
  (Game|OpenLevel(byName) "Game_Over"))

(fn ConstructionScript)