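; Helicopter flyby actor that flies in along -X, hovers briefly, then flies back along +X and destroys itself after a fixed lifespan.
; Tick moves it a fixed step per frame, so speed is frame-rate dependent.
; Flag A flips once X drops below MID (world zero), then a Delay inside Tick holds it before flag B starts the return.
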(event EventBeginPlay
  ;[1 1 1] 生成
  (Actor|SetLifeSpan 15.0) ; 寿命
  (Variables|Default|SetMID 0.0))

(event Collision|EventActorBeginOverlap
  (params (OtherActor :type Actor%20Object%20Reference)))

(event EventTick
  (params (DeltaSeconds :type Float%20%28single-precision%29))
  (bind _returnvalue (Transformation|GetActorLocation))
  (bind _returnvalue_2 (Transformation|GetActorLocation))
  ;[1 1 1] キャラの挙動
  (if (== (Variables|Default|GetA) 0)
    (Transformation|SetActorLocation (Math|Vector|MakeVector (- (.x _returnvalue_2) 1e+01) (.y _returnvalue_2) (.z _returnvalue_2)) false false) ; 移動
    (if (not (>= (.x (Transformation|GetActorLocation)) (Variables|Default|GetMID)))
      (Variables|Default|SetA 1))
    (elif (== (Variables|Default|GetB) 1)
      (Transformation|SetActorLocation (Math|Vector|MakeVector (+ (.x _returnvalue) 1e+01) (.y _returnvalue) (.z _returnvalue)) false false) ; 移動
      (else
        (Utilities|FlowControl|Delay 2.0)
        (Variables|Default|SetB 1)))))

(fn ConstructionScript)