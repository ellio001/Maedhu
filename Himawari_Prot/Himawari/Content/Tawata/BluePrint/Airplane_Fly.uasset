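; Airplane actor that flies in a straight line across the level and destroys itself after a short lifespan.
; On BeginPlay it sets its lifespan and plays an airplane sound cue in 2D.
; Tick waits out a one-second delay before setting flag A, then moves the actor by a fixed negative-X offset every frame, independent of delta time.
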(event EventBeginPlay
  ;[1 1 1] 生成
  (Actor|SetLifeSpan 5.0) ; 寿命
  (Audio|PlaySound2D "/Game/Yafuso/Sound/Airplane_Cue.Airplane_Cue" 1.0 1.0 0.0 0 0))

(event Collision|EventActorBeginOverlap
  (params (OtherActor :type Actor%20Object%20Reference)))

(event EventTick
  (params (DeltaSeconds :type Float%20%28single-precision%29))
  ;[1 1 1] 移動処理
  (if (== (Variables|Default|GetA) 1)
    (Transformation|SetActorLocation (+ (Transformation|GetActorLocation) "-35.000000,0.000000,0.000000") false false) ; 移動
    (else
      (Utilities|FlowControl|Delay 1.0)
      (Variables|Default|SetA 1))))

(fn ConstructionScript)