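; Sparrow actor that flies along negative X while bobbing up and down in a zigzag.
; BeginPlay sets a limited lifespan and records Min and Max height bounds around the spawn altitude.
; Tick steps the location by fixed per-frame amounts without delta time, with flag A flipping the vertical direction whenever a bound is reached.
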(event EventBeginPlay
  ;[1 1 1] 生成
  (Actor|SetLifeSpan 2e+01) ; 寿命
  (Variables|Default|SetMin (- (.z (Transformation|GetActorLocation)) 1e+02))
  (Variables|Default|SetMax (+ (.z (Transformation|GetActorLocation)) 1e+02)))

(event Collision|EventActorBeginOverlap
  (params (OtherActor :type Actor%20Object%20Reference)))

(event EventTick
  (params (DeltaSeconds :type Float%20%28single-precision%29))
  (bind _returnvalue (Transformation|GetActorLocation))
  (bind _returnvalue_2 (Transformation|GetActorLocation))
  ;[1 1 1] キャラの挙動
  (if (== (Variables|Default|GetA) 1)
    (Transformation|SetActorLocation (Math|Vector|MakeVector (- (.x _returnvalue_2) 1e+01) (.y _returnvalue_2) (- (.z _returnvalue_2) 1e+01)) false false) ; 移動
    (if (>= (Variables|Default|GetMin) (.z (Transformation|GetActorLocation)))
      (Variables|Default|SetA 0))
    (else
      (Transformation|SetActorLocation (Math|Vector|MakeVector (- (.x _returnvalue) 1e+01) (.y _returnvalue) (+ (.z _returnvalue) 1e+01)) false false) ; 移動
      (if (>= (.z (Transformation|GetActorLocation)) (Variables|Default|GetMax))
        (Variables|Default|SetA 1)))))

(fn ConstructionScript)